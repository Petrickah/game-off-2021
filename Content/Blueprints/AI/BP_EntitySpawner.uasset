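; Entity spawner that spawns a configurable entity type while BP_CindyCharacter is inside its SpawnerActivation volume.
; Overlap starts a looping cooldown timer that calls SpawnSpiders, which spawns until the count reaches SpawnCap.
; Each spawn uses a random navigable point within the SpawnerArea radius around SpawnerCore, facing along ForwardDirection.
; Leaving the volume clears the timer and resets the count without removing spawned entities.
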(event OnComponentBeginOverlap(SpawnerActivation)
  (params (OverlappedComponent :type Primitive%20Component%20Object%20Reference) (OtherActor :type Actor%20Object%20Reference) (OtherComp :type Primitive%20Component%20Object%20Reference) (OtherBodyIndex :type Integer) (bFromSweep :type Boolean) (SweepResult :type Hit%20Result%20Structure%20%28by%20ref%29))
  (Utilities|Casting|CastToBP_CindyCharacter OtherActor)
  (bind _returnvalue (Utilities|Time|SetTimerbyEvent (delegate Custom|Spawn%20Spiders) (Variables|Default|GetEntity%20Spawn%20Cooldown) true))
  (Variables|Default|SetTimerHandle _returnvalue))

(event OnComponentEndOverlap(SpawnerActivation)
  (params (OverlappedComponent :type Primitive%20Component%20Object%20Reference) (OtherActor :type Actor%20Object%20Reference) (OtherComp :type Primitive%20Component%20Object%20Reference) (OtherBodyIndex :type Integer))
  (Utilities|Casting|CastToBP_CindyCharacter OtherActor)
  (Utilities|Time|ClearandInvalidateTimerbyHandle (Variables|Default|GetTimerHandle))
  (Variables|Default|SetSpawned%20Entities 0))

(event Custom|Spawn%20Spiders
  (if (< (Variables|Default|GetSpawned%20Entities) (Variables|Default|GetSpawn%20Cap))
    (CallFunction|SpawnEntity)
    (Math|Integer|IncrementInt (Variables|Default|GetSpawned%20Entities))))

(fn ConstructionScript)

(fn SpawnEntity
  (Game|SpawnActorfromClass (Variables|Default|GetEntity%20Type) (Math|Transform|MakeTransform (.RandomLocation (Class|NavigationSystemV1|GetRandomPointinNavigableRadius (Transformation|GetWorldLocation (Variables|Default|GetSpawnerCore)) (Variables|/Script/Engine.SphereComponent|GetSphereRadius (Variables|Default|GetSpawnerArea)) 0 "/Script/NavigationSystem.RecastFilter_UseDefaultArea")) (Math|Conversions|RotationFromXVector (Math|Vector|GetForwardVector (Variables|Default|GetForward%20Direction)))) "AlwaysSpawn" 0 0))