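; AI spider enemy character that attacks CindyCharacter on contact and takes point and radial damage.
; Hitbox overlap with a living Cindy plays an attack sound and, after a short delay, applies point damage, with IsAttacking blocking overlapping attacks.
; Incoming damage reduces health, updates IsDead, and launches the spider using a damage-scaled hit vector plus upward lift.
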(event OnComponentBeginOverlap(SpiderHitBox)
  (params (OverlappedComponent :type Primitive%20Component%20Object%20Reference) (OtherActor :type Actor%20Object%20Reference) (OtherComp :type Primitive%20Component%20Object%20Reference) (OtherBodyIndex :type Integer) (bFromSweep :type Boolean) (SweepResult :type Hit%20Result%20Structure%20%28by%20ref%29))
  (bind _ascindy_character (Utilities|Casting|CastToCindyCharacter OtherActor))
  (if (not (Variables|/Script/GameOff2021.CindyCharacter|GetIsDeath _ascindy_character))
    (Audio|Components|Audio|SetSound (Variables|Default|GetSpider%20Sound) (Variables|Default|GetAttack))
    (CallFunction|SpiderAttack _ascindy_character SweepResult)))

(event Custom|Spider%20Attack
  (params (Attacked%20Character :type Cindy%20Character%20Object%20Reference) (Hit :type Hit%20Result%20Structure))
  (if (not (Variables|Default|GetIs%20Attacking))
    (Variables|Default|SetIs%20Attacking true)
    (CallFunction|SpiderStopAttack Attacked%20Character Hit)
    (Audio|Components|Audio|Play (Variables|Default|GetSpider%20Sound) 0.0)))

(event Custom|Spider%20StopAttack
  (params (Attacked%20Character :type Cindy%20Character%20Object%20Reference) (Hit :type Hit%20Result%20Structure))
  (if (Variables|Default|GetIs%20Attacking)
    (Utilities|FlowControl|Delay 0.2)
    (Variables|Default|SetIs%20Attacking false)
    (Game|Damage|ApplyPointDamage Attacked%20Character 5.0 (Math|Vector|Normalize (- (Transformation|GetActorLocation) (Transformation|GetActorLocation Attacked%20Character))) Hit (AI|GetAIController 0) self "/Script/Engine.DamageType")))

(event Game|Damage|EventPointDamage
  (params (Damage :type Float%20%28single-precision%29) (DamageType :type Damage%20Type%20Object%20Reference) (HitLocation :type Vector :default "0, 0, 0") (HitNormal :type Vector :default "0, 0, 0") (HitComponent :type Primitive%20Component%20Object%20Reference) (BoneName :type Name :default "None") (ShotFromDirection :type Vector :default "0, 0, 0") (InstigatedBy :type Controller%20Object%20Reference) (DamageCauser :type Actor%20Object%20Reference) (HitInfo :type Hit%20Result%20Structure%20%28by%20ref%29))
  (bind _returnvalue (* Damage ShotFromDirection))
  (bind (_x _y _z) (Math|Vector|BreakVector _returnvalue))
  (bind _output_get (Variables|Default|SetCurrent%20Health (- (Variables|Default|GetCurrent%20Health) Damage)))
  (Variables|Default|SetIsDead (<= _output_get 0.1))
  (Character|LaunchCharacter (Math|Vector|MakeVector _x _y (+ _z 1e+02)) true true))

(event Game|Damage|EventRadialDamage
  (params (DamageReceived :type Float%20%28single-precision%29) (DamageType :type Damage%20Type%20Object%20Reference) (Origin :type Vector :default "0, 0, 0") (HitInfo :type Hit%20Result%20Structure%20%28by%20ref%29) (InstigatedBy :type Controller%20Object%20Reference) (DamageCauser :type Actor%20Object%20Reference))
  (bind _impactnormal (Collision|BreakHitResult HitInfo))
  (bind _returnvalue (* DamageReceived _impactnormal))
  (bind (_x _y _z) (Math|Vector|BreakVector _returnvalue))
  (bind _output_get (Variables|Default|SetCurrent%20Health (- (Variables|Default|GetCurrent%20Health) DamageReceived)))
  (Variables|Default|SetIsDead (<= _output_get 0.1))
  (Character|LaunchCharacter (Math|Vector|MakeVector _x _y (+ _z 1e+02)) true true))

(fn ConstructionScript)