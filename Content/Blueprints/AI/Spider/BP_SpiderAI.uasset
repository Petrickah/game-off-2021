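; AI controller for the spider enemy that starts its behavior tree when it possesses a BP_SpiderCharacter.
; AI perception updates that involve a CindyCharacter write the sensed state to HasSawTarget and the character to TargetSaw on the Blackboard.
; If that character is dead, it only clears HasSawTarget, and TargetSaw keeps its previous value.
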(event OnTargetPerceptionUpdated(AIPerception)
  (params (Actor :type Actor%20Object%20Reference) (Stimulus :type AI%20Stimulus%20Structure))
  (bind _ascindy_character (Utilities|Casting|CastToCindyCharacter Actor))
  (if (Variables|/Script/GameOff2021.CindyCharacter|GetIsDeath _ascindy_character)
    (AI|Components|Blackboard|SetValueasBool (Variables|Default|GetBlackboard) (Utilities|Name|MakeLiteralName "HasSawTarget") false)
    (else
      (AI|Components|Blackboard|SetValueasBool (Variables|Default|GetBlackboard) (Utilities|Name|MakeLiteralName "HasSawTarget") (.bSuccessfullySensed (Utilities|Struct|BreakAIStimulus Stimulus)))
      (AI|Components|Blackboard|SetValueasObject (Variables|Default|GetBlackboard) (Utilities|Name|MakeLiteralName "TargetSaw") _ascindy_character))))

(event EventPossess
  (params (PossessedPawn :type Pawn%20Object%20Reference))
  (Utilities|Casting|CastToBP_SpiderCharacter PossessedPawn)
  (AI|RunBehaviorTree (Variables|/Script/AIModule.BehaviorTreeComponent|GetDefaultBehaviorTreeAsset (Variables|Default|GetBehaviorTree))))

(fn ConstructionScript)