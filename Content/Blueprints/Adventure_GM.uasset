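; Adventure game mode Blueprint that handles pausing, resuming and quitting the game through a pause menu.
; On pause it lazily creates and reuses the BP_PauseMenu widget, switches to UI-only input with the cursor shown, pauses the game and focuses the Resume button.
; Resume restores game-only input, hides the cursor and removes the menu, while exit quits; both act only while paused.
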(event Custom|On%20Game%20Pause
  (bind _returnvalue (Game|GetPlayerController 0))
  (Utilities|IsValid (Variables|Default|GetPause%20Menu)
    (:Is%20Valid
      _)
    (:Is%20Not%20Valid
      (bind _returnvalue_2 (UserInterface|CreateWidget "/Game/Blueprints/BP_PauseMenu.BP_PauseMenu_C"))
      (Variables|Default|SetPause%20Menu _returnvalue_2)))
  (Variables|/Script/Engine.PlayerController|SetbShowMouseCursor _returnvalue true)
  (Input|SetInputModeUIOnly _returnvalue (Variables|Default|GetPause%20Menu) "LockOnCapture")
  (UserInterface|Viewport|AddtoViewport (Variables|Default|GetPause%20Menu) 0)
  (Game|SetGamePaused true)
  (Widget|SetFocus (Variables|/Game/Blueprints/BP_PauseMenu.BP_PauseMenu_C|GetResumeButton (Variables|Default|GetPause%20Menu))))

(event Custom|On%20Game%20Resume
  (bind _returnvalue (Game|GetPlayerController 0))
  (if (Game|IsGamePaused)
    (Input|SetInputModeGameOnly _returnvalue)
    (Variables|/Script/Engine.PlayerController|SetbShowMouseCursor _returnvalue false)
    (Widget|RemovefromParent (Variables|Default|GetPause%20Menu))
    (Game|SetGamePaused false)))

(event Custom|On%20Game%20Exit
  (if (Game|IsGamePaused)
    (Game|QuitGame 0 "Quit" false)))

(fn ConstructionScript)