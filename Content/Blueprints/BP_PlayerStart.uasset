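; BP_PlayerStart is the respawn point for the player's BP_CindyCharacter.
; On BeginPlay it stores itself in the PlayerStart reference of the current player pawn, if that pawn is a BP_CindyCharacter.
; OnReset waits briefly, spawns ActorClass at its own transform and has the first player controller possess the new pawn.
; It then passes itself to the new character through OnRespawn.
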(event EventBeginPlay
  (|CallParentFunction)
  (bind _asbp_cindy_character (Utilities|Casting|CastToBP_CindyCharacter (Game|Player|GetPlayerPawn 0)))
  (Variables|/Game/Blueprints/BP_CindyCharacter.BP_CindyCharacter_C|SetPlayerStart _asbp_cindy_character self))

(event EventOnReset
  (Utilities|FlowControl|Delay 0.5)
  (bind _returnvalue (Game|SpawnActorfromClass (Variables|Default|GetActor%20Class) (Transformation|GetActorTransform) "Undefined" 0 0))
  (bind _aspawn (Utilities|Casting|CastToPawn _returnvalue))
  (Pawn|Possess (Game|GetPlayerController 0) _aspawn)
  (bind _asbp_cindy_character (Utilities|Casting|CastToBP_CindyCharacter _aspawn))
  (Class|CindyCharacter|OnRespawn _asbp_cindy_character self))

(fn ConstructionScript)