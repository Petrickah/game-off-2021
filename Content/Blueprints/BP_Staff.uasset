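; BP_Staff is the staff weapon that handles equip montage, magic circle attachment and four elemental spells for its owning character.
; CastSpell calls its parent, then, if casting, plays the matching montage.
; A shared SpellDelay macro times the release from montage length and derives a transform from mesh and camera boom.
; Fire and Water then spawn projectiles, while Lightning and Arcane only call StopMovement(false) and stop their montage.
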(event Custom|Fire%20Spell
  (bind _returnvalue (Animation|PlayAnimMontage (Variables|Default|GetStaffOwner) "/Game/Blueprints/Montages/FireSpell.FireSpell" 1.0 "None"))
  (bind (_character _relative_transform) (Utilities|SpellDelay _returnvalue 0.35 (Variables|Default|GetStaffMesh))
    (:executeOut
      (Utilities|CastSpell _character "/Game/Blueprints/Montages/FireSpell.FireSpell" "/Game/FXVarietyPack/Blueprints/BP_ky_fireBall.BP_ky_fireBall_C" _relative_transform))))

(event Custom|Water%20Spell
  (bind _returnvalue (Animation|PlayAnimMontage (Variables|Default|GetStaffOwner) "/Game/Blueprints/Montages/WaterSpell.WaterSpell" 1.0 "None"))
  (bind (_character _relative_transform) (Utilities|SpellDelay _returnvalue 0.35 (Variables|/Script/Engine.Character|GetMesh (Variables|Default|GetStaffOwner)))
    (:executeOut
      (Utilities|CastSpell _character "/Game/Blueprints/Montages/WaterSpell.WaterSpell" "/Game/FXVarietyPack/Blueprints/BP_ky_waterBall.BP_ky_waterBall_C" _relative_transform))))

(event Custom|Lightning%20Spell
  (bind _returnvalue (Animation|PlayAnimMontage (Variables|Default|GetStaffOwner) "/Game/Blueprints/Montages/LightningSpell.LightningSpell" 1.0 "None"))
  (bind _character (Utilities|SpellDelay _returnvalue 0.0 (Variables|/Script/Engine.Character|GetMesh (Variables|Default|GetStaffOwner)))
    (:executeOut
      (Utilities|FlowControl|Sequence
        (:then_0
          (Class|CindyCharacter|StopMovement _character false))
        (:then_1
          (Animation|StopAnimMontage _character "/Game/Blueprints/Montages/LightningSpell.LightningSpell"))))))

(event Custom|Arcane%20Spell
  (bind _returnvalue (Animation|PlayAnimMontage (Variables|Default|GetStaffOwner) "/Game/Blueprints/Montages/ArcaneSpell.ArcaneSpell" 1.0 "None"))
  (bind _character (Utilities|SpellDelay _returnvalue 0.0 (Variables|/Script/Engine.Character|GetMesh (Variables|Default|GetStaffOwner)))
    (:executeOut
      (Utilities|FlowControl|Sequence
        (:then_0
          (Class|CindyCharacter|StopMovement _character false))
        (:then_1
          (Animation|StopAnimMontage _character "/Game/Blueprints/Montages/ArcaneSpell.ArcaneSpell"))))))

(event EventEquippingStaff
  (params (StaffOwner :type Cindy%20Character%20Object%20Reference))
  (Class|CindyCharacter|StopMovement StaffOwner true)
  (bind _returnvalue (Animation|PlayAnimMontage StaffOwner "/Game/Blueprints/Montages/EquippingStaff.EquippingStaff" 1.0 "Default"))
  (Utilities|FlowControl|Delay _returnvalue)
  (Class|MagicalStaff|DestroyEffect StaffOwner)
  (Variables|Default|SetStaffOwner StaffOwner))

(event EventShowMagic
  (params (StaffOwner :type Cindy%20Character%20Object%20Reference) (RelativeTransform :type Transform))
  (bind _returnvalue (AddComponent|AddChildActorComponent StaffOwner false RelativeTransform))
  (Variables|/Script/GameOff2021.CindyCharacter|SetMagicCircle StaffOwner _returnvalue))

(event EventStopMontage
  (params (Montage :type Anim%20Montage%20Object%20Reference) (Interrupted :type Boolean))
  (if (not Interrupted)
    (Animation|StopAnimMontage (Variables|Default|GetStaffOwner) Montage)
    (Variables|Default|SetIsAttacking false)))

(event EventCastSpell
  (params (StaffOwner :type Cindy%20Character%20Object%20Reference) (SpellType :type ESpellType%20Enum :default "None"))
  (bind _output_get (Variables|Default|SetStaffOwner StaffOwner))
  (|CallParentFunction _output_get SpellType)
  (if (Variables|Default|GetIsCasting)
    (switch Utilities|FlowControl|Switch|SwitchonESpellType SpellType
      (:Fire
        (CallFunction|FireSpell))
      (:Water
        (CallFunction|WaterSpell))
      (:Lightning
        (CallFunction|LightningSpell))
      (:Arcane
        (CallFunction|ArcaneSpell)))))

(fn ConstructionScript)