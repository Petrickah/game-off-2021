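; PlaySOundNotify is an animation notify state that plays a configurable sound for the duration of its window.
; On begin it assigns the sound to BP_CindyCharacter's audio component and plays it from a slight start offset; on end it stops that component.
; A shared helper finds the component through player pawn 0 rather than the animated mesh's owner, and flags failure if the cast fails.
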(fn ReceivedNotifyBegin
  (params (MeshComp :type Skeletal%20Mesh%20Component%20Object%20Reference) (Animation :type Anim%20Sequence%20Base%20Object%20Reference) (TotalDuration :type Float%20%28single-precision%29))
  (bind (_audio_component _isfailed) (CallFunction|GetAudioComponent MeshComp))
  (if (not _isfailed)
    (Audio|Components|Audio|SetSound _audio_component (Variables|Default|GetSound))
    (Audio|Components|Audio|Play _audio_component 0.2)
    (return false)))

(fn GetAudioComponent
  (params (Mesh :type Skeletal%20Mesh%20Component%20Object%20Reference))
  (bind _asbp_cindy_character (Utilities|Casting|CastToBP_CindyCharacter (Game|Player|GetPlayerPawn Mesh))
    (:then
      (LocalVariables|SetIsCastFailed false))
    (:CastFailed
      (LocalVariables|SetIsCastFailed true)))
  (return (Variables|/Game/Blueprints/BP_CindyCharacter.BP_CindyCharacter_C|GetAudioComponent _asbp_cindy_character) (LocalVariables|GetIsCastFailed)))

(fn ReceivedNotifyEnd
  (params (MeshComp :type Skeletal%20Mesh%20Component%20Object%20Reference) (Animation :type Anim%20Sequence%20Base%20Object%20Reference))
  (bind (_audio_component _isfailed) (CallFunction|GetAudioComponent MeshComp))
  (if (not _isfailed)
    (Audio|Components|Audio|Stop _audio_component)
    (return false)))