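; BPC_FireSpell is a spell component that casts a fireball from a staff.
; On BeginPlay it binds its cast handler through AssignCastSpellEvent.
; A cast plays the FireSpell montage on the staff owner, waits for a delay derived from it, then spawns BP_FireBall at a staff mesh socket transform.
; A valid projectile receives SpellDamage through OnCastSpell, then the spell is stopped.
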(event Custom|Cast%20FireSpell
  (params (Staff%20Owner :type Cindy%20Character%20Object%20Reference))
  (bind _returnvalue (Animation|PlayAnimMontage Staff%20Owner "/Game/Blueprints/Montages/FireSpell.FireSpell" 1.0 "None"))
  (bind _duration (CallFunction|SpellDelay _returnvalue))
  (Utilities|FlowControl|Delay _duration)
  (bind _relative_transform (CallFunction|CalculateSocket (Variables|/Script/GameOff2021.MagicalStaff|GetStaffMesh (Variables|Default|GetStaff))))
  (bind _spell_actor (CallFunction|CastSpell "/Game/Blueprints/Spells/BP_FireBall.BP_FireBall_C" _relative_transform))
  (Utilities|IsValid _spell_actor
    (:Is%20Valid
      (bind _asbp_magic_projectile (Utilities|Casting|CastToBP_MagicProjectile _spell_actor))
      (Default|OnCastSpell _asbp_magic_projectile (Variables|Default|GetSpell%20Damage))
      (CallFunction|StopSpell Staff%20Owner "/Game/Blueprints/Montages/FireSpell.FireSpell"))))

(event EventBeginPlay
  (EventDispatchers|AssignCastSpellEvent (delegate Custom|Cast%20FireSpell)))