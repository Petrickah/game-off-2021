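; Magic spell projectile that deals area damage and plays an impact sound.
; On cast, it scales base spell damage by the incoming damage factor and a multiplier.
; When the AreaOfEffect sphere begins an overlap, it applies radial damage with falloff, using the sphere radius as the inner radius and player 0's controller as instigator.
; The construction script assigns the configurable Sound to the impact audio component.
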(event OnComponentBeginOverlap(AreaOfEffect)
  (params (OverlappedComponent :type Primitive%20Component%20Object%20Reference) (OtherActor :type Actor%20Object%20Reference) (OtherComp :type Primitive%20Component%20Object%20Reference) (OtherBodyIndex :type Integer) (bFromSweep :type Boolean) (SweepResult :type Hit%20Result%20Structure%20%28by%20ref%29))
  (Class|GameplayStatics|ApplyRadialDamagewithFalloff (Variables|Default|GetFinal%20Damage) 2.0 (Transformation|GetActorLocation) (Variables|/Script/Engine.SphereComponent|GetSphereRadius (Variables|Default|GetAreaOfEffect)) 2.5e+02 0.2 "/Script/Engine.DamageType" 0 self (Game|GetPlayerController 0) "ECC_Pawn")
  (Audio|Components|Audio|Play (Variables|Default|GetImpact%20Sound) 0.0))

(event Custom|On%20Cast%20Spell
  (params (Spell%20Damage%20Factor :type Float%20%28single-precision%29))
  (Variables|Default|SetFinal%20Damage (* (+ (* Spell%20Damage%20Factor (Variables|Default|GetBase%20Spell%20Damage)) (Variables|Default|GetBase%20Spell%20Damage)) (Variables|Default|GetDamage%20Multiplier))))

(fn ConstructionScript
  (|CallParentFunction)
  (Audio|Components|Audio|SetSound (Variables|Default|GetImpact%20Sound) (Variables|Default|GetSound)))