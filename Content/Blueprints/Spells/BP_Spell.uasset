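; BP_Spell provides shared casting logic for spells owned by a BP_Staff.
; On cast it runs the parent handler, then, if unlocked, caches the staff and its wielder, updates the mana message and calls the cast event.
; Helper functions spawn spell actors with the wielder as Instigator, stop movement and montages, offset duration by SyncSpell, and get a transform from the staff using the Cindy character's camera boom.
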(event EventOnCastSpell
  (params (ManaAmmount :type Float%20%28single-precision%29))
  (|CallParentFunction ManaAmmount)
  (if (Variables|Default|GetIsUnlocked)
    (CallFunction|IndentifyStaff)
    (Class|BPISorceress|UpdateMana(Message) (Variables|Default|GetStaff) (Variables|Default|GetManaRemaining))
    (Default|CallCastSpellEvent (Variables|Default|GetStaffOwner))))

(fn CastSpell
  (params (Actor%20Class :type Actor%20Class%20Reference) (Spawn%20Transform :type Transform))
  (bind _returnvalue (Game|SpawnActorfromClass Actor%20Class Spawn%20Transform "Undefined" 0 (Variables|Default|GetStaffOwner)))
  (return _returnvalue))

(fn StopSpell
  (params (Character :type Cindy%20Character%20Object%20Reference) (Anim%20Montage :type Anim%20Montage%20Object%20Reference))
  (Utilities|FlowControl|Sequence
    (:then_0
      (Class|CindyCharacter|StopMovement Character false))
    (:then_1
      (Animation|StopAnimMontage Character Anim%20Montage))))

(fn IndentifyStaff
  (bind _asbp_staff (Utilities|Casting|CastToBP_Staff (Components|GetOwner)))
  (Variables|Default|SetStaff _asbp_staff)
  (Variables|Default|SetStaffOwner (Variables|/Game/Blueprints/BP_Staff.BP_Staff_C|GetStaffOwner _asbp_staff)))

(fn SpellDelay
  (params (Spell%20Duration :type Float%20%28single-precision%29))
  (return (- Spell%20Duration (Variables|SpellProperties|GetSync%20Spell))))

(fn CalculateSocket
  (params (Mesh :type Skeletal%20Mesh%20Component%20Object%20Reference))
  (bind _asbp_cindy_character (Utilities|Casting|CastToBP_CindyCharacter (Variables|Default|GetStaffOwner)))
  (return (Class|MagicalStaff|GetRelativeTransform (Variables|Default|GetStaff) Mesh (Variables|/Game/Blueprints/BP_CindyCharacter.BP_CindyCharacter_C|GetCameraBoom _asbp_cindy_character))))